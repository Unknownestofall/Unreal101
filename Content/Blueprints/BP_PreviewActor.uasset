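; BP_PreviewActor is a placement preview actor that shows a mesh and signals whether its spawn location is valid.
; Separate events apply its stored variables to the preview mesh component: the static mesh, the collision mode, and a valid or invalid material based on IsValidSpawn.
; Another event restores a default material chosen by index from an array, always on the first material slot.
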(event Custom|SetDefaultMaterial
  ;[0.15 0.15 0.15 0.5] Setting Default Mat
  (Rendering|Material|SetMaterial (Variables|Default|GetSM_PreviewMesh) 0 (Utilities|Array|Get(acopy) (Variables|Default|GetDefaultMaterials) (Variables|Default|GetdefaultMaterialIndex))))

(event Custom|SwitchMaterial
  (bind _sm_previewmesh (Variables|Default|GetSM_PreviewMesh))
  ;[0.15 0.15 0.15 0.5] Changing Material
  (if (Variables|Default|GetisValidSpawn)
    (Rendering|Material|SetMaterial _sm_previewmesh 0 (Variables|Default|GetValidMaterial))
    (else
      (Rendering|Material|SetMaterial _sm_previewmesh 0 (Variables|Default|GetInvalidMaterial)))))

(event Custom|SwitchPreviewMesh
  ;[0.15 0.15 0.15 0.5] setting Static Mesh
  (Components|StaticMesh|SetStaticMesh (Variables|Default|GetSM_PreviewMesh) (Variables|Default|GetPreviewObjects)))

(event Custom|SwitchCollisionType
  ;[0.15 0.15 0.15 0.5] Enable Collisions
  (Collision|SetCollisionEnabled (Variables|Default|GetSM_PreviewMesh) (Variables|Default|GetcollisionType)))

(fn ConstructionScript)